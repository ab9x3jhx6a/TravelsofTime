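; Main menu actor with Start, Exit and Credits buttons built from components in the world rather than UMG.
; Start opens "level1" and Exit quits the game, while the Credits click handler is empty.
; Cursor-over events swap each button's material between normal and hover versions.
; BeginPlay toggles the root component's visibility without propagating to its children.
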(event `self.ReceiveBeginPlay`)

(event `self.ReceiveActorBeginOverlap`
  (params (OtherActor :type "Actor Object Reference")))

(event `self.ReceiveTick`
  (params (DeltaSeconds :type "Float (single-precision)")))

(event `self.ReceiveBeginPlay`
  (`SceneComponent.ToggleVisibility` (`self.DefaultSceneRoot`) false))

(event `self.Start_Btn.OnClicked`
  (params (TouchedComponent :type "PrimitiveComponent Object Reference"))
  (`GameplayStatics.OpenLevel` "level1"))

(event `self.Exit_Btn.OnClicked`
  (params (TouchedComponent :type "PrimitiveComponent Object Reference"))
  (`KismetSystemLibrary.QuitGame` null "Quit"))

(event `self.Credits_Btn.OnClicked`
  (params (TouchedComponent :type "PrimitiveComponent Object Reference")))

(event `self.Credits_Btn.OnBeginCursorOver`
  (params (TouchedComponent :type "PrimitiveComponent Object Reference"))
  (`PrimitiveComponent.SetMaterial` (`self.Credits_Btn`) 0 "/Game/Assets/Materials/Button_hover.Button_hover"))

(event `self.Credits_Btn.OnEndCursorOver`
  (params (TouchedComponent :type "PrimitiveComponent Object Reference"))
  (`PrimitiveComponent.SetMaterial` (`self.Credits_Btn`) 0 "/Game/Assets/Materials/Button_Mat.Button_Mat"))

(event `self.Exit_Btn.OnBeginCursorOver`
  (params (TouchedComponent :type "PrimitiveComponent Object Reference"))
  (`PrimitiveComponent.SetMaterial` (`self.Exit_Btn`) 0 "/Game/Assets/Materials/Button_hover.Button_hover"))

(event `self.Exit_Btn.OnEndCursorOver`
  (params (TouchedComponent :type "PrimitiveComponent Object Reference"))
  (`PrimitiveComponent.SetMaterial` (`self.Exit_Btn`) 0 "/Game/Assets/Materials/Button_Mat.Button_Mat"))

(event `self.Start_Btn.OnBeginCursorOver`
  (params (TouchedComponent :type "PrimitiveComponent Object Reference"))
  (`PrimitiveComponent.SetMaterial` (`self.Start_Btn`) 0 "/Game/Assets/Materials/Button_hover.Button_hover"))

(event `self.Start_Btn.OnEndCursorOver`
  (params (TouchedComponent :type "PrimitiveComponent Object Reference"))
  (`PrimitiveComponent.SetMaterial` (`self.Start_Btn`) 0 "/Game/Assets/Materials/Button_Mat.Button_Mat"))

(fn `UserConstructionScript`)