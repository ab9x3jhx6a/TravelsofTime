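; End door Blueprint that holds two door halves open and loads a named level when its box trigger is overlapped.
; BeginPlay stores each half's start location, and Tick sets both to offsets in opposite X directions from those positions.
; The Tick branch condition is fixed to true, so the closed-state path never runs and the doors snap open without interpolation.
; Any overlap with the box opens LevelName, with no actor filter.
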(event `self.ReceiveBeginPlay`
  ;[1 1 1] Save inital state
  (set `self.DoorLStart` (`SceneComponent.K2_GetComponentLocation` (`self.DoorL`)))
  (set `self.DoorRStart` (`SceneComponent.K2_GetComponentLocation` (`self.DoorR`))))

(event `self.ReceiveTick`
  (params (DeltaSeconds :type "Float (single-precision)"))
  ;[1 1 1] Change gate state on switch
  (if true
    (`SceneComponent.K2_SetWorldLocation` (`self.DoorL`) (+ (`self.DoorLStart`) (-200.0 0.0 0.0)) false false)
    (`SceneComponent.K2_SetWorldLocation` (`self.DoorR`) (+ (`self.DoorRStart`) (200.0 0.0 0.0)) false false)
    (else
      (`SceneComponent.K2_SetWorldLocation` (`self.DoorL`) (`self.DoorLStart`) false false)
      (`SceneComponent.K2_SetWorldLocation` (`self.DoorR`) (`self.DoorRStart`) false false))))

(event `self.Box.OnComponentBeginOverlap`
  (params (OtherActor :type "Actor Object Reference") (OtherComp :type "PrimitiveComponent Object Reference") (OtherBodyIndex :type Integer) (bFromSweep :type Boolean) (SweepResult :type "HitResult Structure (by ref)"))
  (`GameplayStatics.OpenLevel` (`self.LevelName`)))

(fn `UserConstructionScript`)